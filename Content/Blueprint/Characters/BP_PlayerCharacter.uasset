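; Player character Blueprint that adds a cooldown-limited dash in the actor's forward direction.
; The dash input saves velocity, triggers a small jump with a temporary jump velocity and sets horizontal speed.
; After the dash duration it restores the saved horizontal velocity and jump velocity, then re-enables dashing when the cooldown ends.
; Pressing W reloads the current level, and RotateBeforeAction always returns false.
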(event `EnhancedInput|/Game/Inputs/InputActions/IA_Dash`
  (params (ActionValue :type Boolean) (ElapsedSeconds :type "Float (double-precision)") (TriggeredSeconds :type "Float (double-precision)") (InputAction :type "InputAction Object Reference" :default "/Game/Inputs/InputActions/IA_Dash.IA_Dash"))
  (:`Triggered`
    (`self.HandleDash`)))

(event `HandleDash`
  (bind _charactermovement (`self.CharacterMovement`))
  (bind _dashduration (`self.DashDuration`))
  (bind _charactermovement_2 (`self.CharacterMovement`))
  (bind (_returnvalue_x _returnvalue_y) (`KismetMathLibrary.BreakVector` (* (`self.GetActorForwardVector`) (`self.DashSpeed`))))
  (bind (_velocity_x _velocity_y) (`KismetMathLibrary.BreakVector` (`MovementComponent.Velocity` _charactermovement_2)))
  ;[1 1 1] Comment
  (if (`self.CanDash`)
    (set `self.CanDash` false)
    (set `self.OldVelocity` (`KismetMathLibrary.MakeVector` _velocity_x _velocity_y))
    (set `self.OldJumpVelocity` (`CharacterMovementComponent.JumpZVelocity` _charactermovement_2))
    (set `CharacterMovementComponent.JumpZVelocity` 200.0 _charactermovement_2) ; Tested, dont change
    (`self.Jump`)
    (set `MovementComponent.Velocity` (`KismetMathLibrary.MakeVector` _returnvalue_x _returnvalue_y) (`self.CharacterMovement`))
    (`KismetSystemLibrary.Delay` _dashduration)
    (`self.StopJumping`)
    (set `MovementComponent.Velocity` (`self.OldVelocity`) _charactermovement)
    (set `CharacterMovementComponent.JumpZVelocity` (`self.OldJumpVelocity`) _charactermovement)
    (`KismetSystemLibrary.Delay` (- (`self.DashCooldown`) _dashduration))
    (set `self.CanDash` true)))

(event `Key|W`
  (params (Key :type "Key Structure"))
  (:`Pressed`
    (bind _returnvalue (`GameplayStatics.GetCurrentLevelName` true))
    (`GameplayStatics.OpenLevel` (`KismetStringLibrary.Conv_StringToName` _returnvalue))))

(fn `RotateBeforeAction`
  (returns (MustRotate :type Boolean))
  (return false))

(fn `UserConstructionScript`)