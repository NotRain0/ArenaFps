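; BP_BaseEnemy is an enemy character that makes a melee attack when the player is close.
; It caches the first player-class actor on BeginPlay and checks its distance every Tick.
; A CanAttack flag gates the attack, in which one timeline pitches the Arm forward and a second returns it.
; Damage goes through the player's ChangeHealth only if still in range when the first swing finishes.
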(event `self.ReceiveBeginPlay`
  (bind _outactors (`GameplayStatics.GetAllActorsOfClass` "/Script/ArenaFps.PlayerClass"))
  (set `self.PlayerRef` (`|GetArrayItem` _outactors))
  (set `self.canAttack` true))

(event `self.ReceiveTick`
  (params (DeltaSeconds :type "Float (single-precision)"))
  (bind _playerref (`self.PlayerRef`))
  (`/Engine/EditorBlueprintResources/StandardMacros.IsValid` _playerref
    (:`Is Valid`
      (if (<= (`self.GetDistanceTo` _playerref self) 100.0)
        (`self.AttackCustom`)))))

(event `AttackCustom`
  (bind _playerref (`self.PlayerRef`))
  (if (`self.canAttack`)
    (set `self.canAttack` false)
    (bind (_direction _newtrack_0) (`Timeline|Timeline` :!via `PlayFromStart`)
      (:`Update`
        (`SceneComponent.K2_SetRelativeRotation` (`self.Arm`) (`KismetMathLibrary.MakeRotator` 0.0 _newtrack_0) false false))
      (:`Finished`
        (`/Engine/EditorBlueprintResources/StandardMacros.IsValid` _playerref
          (:`Is Valid`
            (if (<= (`self.GetDistanceTo` _playerref self) 100.0)
              (`self.ChangeHealth` (`self.PlayerRef`) -25)
              (bind (_direction_2 _newtrack_0_2) (`Timeline|Timeline_0` :!via `PlayFromStart` :!label _label)
                (:`Update`
                  (`SceneComponent.K2_SetRelativeRotation` (`self.Arm`) (`KismetMathLibrary.MakeRotator` 0.0 _newtrack_0_2) false false))
                (:`Finished`
                  (set `self.canAttack` true)))
              (else
                (goto _label :!via `PlayFromStart`)))))))))

(fn `UserConstructionScript`)