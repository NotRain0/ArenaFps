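; Player character Blueprint handling dash, procedural arm animation and a level restart key.
; Dash sets horizontal velocity from movement input with a small temporary jump, then restores saved velocity and jump strength, gated by a cooldown.
; Timelines drive left and right arm pitch; weapon reload stops them, rotates the Scene component and fades a hand color material parameter.
; Pressing W reopens the current level, and RotateBeforeAction always returns false.
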(event `EnhancedInput|/Game/Inputs/InputActions/IA_Dash`
  (params (ActionValue :type Boolean) (ElapsedSeconds :type "Float (double-precision)") (TriggeredSeconds :type "Float (double-precision)") (InputAction :type "InputAction Object Reference" :default "/Game/Inputs/InputActions/IA_Dash.IA_Dash"))
  ;[1 1 1] Comment
  ;;[0 0 0 0.5] Comment
  (:`Triggered`
    (`self.HandleDash`)))

(event `HandleDash`
  (bind _charactermovement (`self.CharacterMovement`))
  (bind _dashduration (`self.DashDuration`))
  (bind (_movementvector_x _movementvector_y) (`KismetMathLibrary.BreakVector2D` (`self.MovementVector`)))
  (bind _charactermovement_2 (`self.CharacterMovement`))
  (bind (_velocity_x _velocity_y) (`KismetMathLibrary.BreakVector` (`MovementComponent.Velocity` _charactermovement_2)))
  (bind (_returnvalue_x _returnvalue_y) (`KismetMathLibrary.BreakVector` (* (`KismetMathLibrary.Normal` (+ (* _movementvector_x (`self.GetActorRightVector`)) (* _movementvector_y (`self.GetActorForwardVector`)))) (`self.DashSpeed`))))
  ;[1 1 1] Comment
  (if (`self.CanDashBP`)
    (set `self.CanDashBP` false)
    (set `self.OldVelocity` (`KismetMathLibrary.MakeVector` _velocity_x _velocity_y))
    (set `self.OldJumpVelocity` (`CharacterMovementComponent.JumpZVelocity` _charactermovement_2))
    (set `CharacterMovementComponent.JumpZVelocity` 200.0 _charactermovement_2) ; Tested, dont change
    (`self.Jump`)
    (set `MovementComponent.Velocity` (`KismetMathLibrary.MakeVector` _returnvalue_x _returnvalue_y) (`self.CharacterMovement`))
    (`KismetSystemLibrary.Delay` _dashduration)
    (`self.StopJumping`)
    (set `MovementComponent.Velocity` (`self.OldVelocity`) _charactermovement)
    (set `CharacterMovementComponent.JumpZVelocity` (`self.OldJumpVelocity`) _charactermovement)
    (`KismetSystemLibrary.Delay` (- (`self.DashCooldown`) _dashduration))
    (set `self.CanDashBP` true)))

(event `Key|W`
  (params (Key :type "Key Structure"))
  ; Comment
  (:`Pressed`
    (bind _returnvalue (`GameplayStatics.GetCurrentLevelName` true))
    (`GameplayStatics.OpenLevel` (`KismetStringLibrary.Conv_StringToName` _returnvalue))))

(event `self.ReloadFirstWeaponBlueprint`
  (`|ExecutionSequence`
    (:`then_0`
      (bind (_direction _newtrack_0) (`Timeline|Timeline_1` :!via `Stop` :!label _label)
        (:`Update`
          (`SceneComponent.K2_SetRelativeRotation` (`self.LArm`) (`KismetMathLibrary.MakeRotator` -135.0 _newtrack_0) false false))))
    (:`then_1`
      (bind (_direction_2 _newtrack_0_2) (`Timeline|Timeline_2` :!via `Stop` :!label _label_2)
        (:`Update`
          (`SceneComponent.K2_SetRelativeRotation` (`self.RArm`) (`KismetMathLibrary.MakeRotator` 135.0 _newtrack_0_2) false false))))
    (:`then_2`
      (bind (_direction_3 _newtrack_0_3) (`Timeline|Timeline` :!via `PlayFromStart`)
        (:`Update`
          (`SceneComponent.K2_SetRelativeRotation` (`self.Scene`) (`KismetMathLibrary.MakeRotator` _newtrack_0_3 _newtrack_0_3 _newtrack_0_3) false false))
        (:`Finished`
          (`SceneComponent.K2_SetRelativeRotation` (`self.Scene`) (`KismetMathLibrary.MakeRotator` 0.0) false false))))
    (:`then_3`
      (bind (_direction_4 _newtrack_0_4) (`Timeline|Timeline_0` :!via `PlayFromStart`)
        (:`Update`
          (`MaterialInstanceDynamic.SetScalarParameterValue` (`self.DynamicMaterialInstance`) "HandColorParam" (`KismetMathLibrary.Lerp` 0.0 1.0 _newtrack_0_4)))))))

(event `self.AnimateLeftHand`
  (goto _label :!via `PlayFromStart`))

(event `self.AnimateRightHand`
  (goto _label_2 :!via `PlayFromStart`))

(fn `RotateBeforeAction`
  (returns (MustRotate :type Boolean))
  (return false))

(fn `UserConstructionScript`)