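; Turret Blueprint that registers BP_BaseEnemy actors in its Sphere overlap and drops them on exit, clearing the current target.
; Fire spawns a BP_TurretProjectile at the Cylinder, directed along the Cube's forward vector with random X/Y spread, gated by a short cooldown.
; The logic that picks the first valid target, rotates the Cube toward it and calls Fire is disconnected, as Tick is empty.
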(event `self.ReceiveTick`
  (params (DeltaSeconds :type "Float (single-precision)")))

(event `self.Sphere.OnComponentBeginOverlap`
  (params (OverlappedComponent :type "PrimitiveComponent Object Reference") (OtherActor :type "Actor Object Reference") (OtherComp :type "PrimitiveComponent Object Reference") (OtherBodyIndex :type Integer) (bFromSweep :type Boolean) (SweepResult :type "HitResult Structure (by ref)"))
  (bind _targetarray (`self.TargetArray`))
  (bind _asbp_base_enemy (cast `/Game/Blueprint/Characters/BP_BaseEnemy` OtherActor))
  (if (not (`KismetArrayLibrary.Array_Contains` _targetarray _asbp_base_enemy))
    (`KismetArrayLibrary.Array_Add` _targetarray _asbp_base_enemy)))

(event `self.Sphere.OnComponentEndOverlap`
  (params (OverlappedComponent :type "PrimitiveComponent Object Reference") (OtherActor :type "Actor Object Reference") (OtherComp :type "PrimitiveComponent Object Reference") (OtherBodyIndex :type Integer))
  (bind _targetarray (`self.TargetArray`))
  (`/Engine/EditorBlueprintResources/StandardMacros.IsValid` OtherActor
    (:`Is Valid`
      (bind _asbp_base_enemy (cast `/Game/Blueprint/Characters/BP_BaseEnemy` OtherActor))
      (if (`KismetArrayLibrary.Array_Contains` _targetarray _asbp_base_enemy)
        (`KismetArrayLibrary.Array_RemoveItem` _targetarray _asbp_base_enemy)
        (set `self.CurrentTarget` null)))))

(event `Fire`
  (bind (_returnvalue_x _returnvalue_y _returnvalue_z) (`KismetMathLibrary.BreakVector` (`SceneComponent.GetForwardVector` (`self.Cube`))))
  (bind (_returnvalue_location _returnvalue_rotation) (`KismetMathLibrary.BreakTransform` (`SceneComponent.K2_GetComponentToWorld` (`self.Cylinder`))))
  (if (`self.CanFire`)
    (set `self.CanFire` false)
    (bind _returnvalue (`|SpawnActorFromClass` "/Game/Blueprint/Projectile/BP_TurretProjectile.BP_TurretProjectile_C" (`KismetMathLibrary.MakeTransform` _returnvalue_location _returnvalue_rotation) "Undefined" "MultiplyWithRoot" null null))
    (`/Engine/EditorBlueprintResources/StandardMacros.IsValid` _returnvalue
      (:`Is Valid`
        (set `BaseProjectile.ProjectileDirection` (`KismetMathLibrary.MakeVector` (+ _returnvalue_x (`KismetMathLibrary.RandomFloatInRange` -5.0 5.0)) (+ (`KismetMathLibrary.RandomFloatInRange` -5.0 5.0) _returnvalue_y) _returnvalue_z) _returnvalue)
        (`KismetSystemLibrary.Delay` 0.1)
        (set `self.CanFire` true)))))

(fn `UserConstructionScript`)