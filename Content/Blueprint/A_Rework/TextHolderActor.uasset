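; TextHolderActor is a world-space damage text actor that turns to face the player every tick.
; While ParentScene is valid, it rotates that component fully toward PlayerRef.
; Otherwise it rotates WidgetHolder with pitch held at zero and, once only, starts two timelines on DmgWidget: a reversed one driving scale and another driving render opacity.
; The actor destroys itself when the opacity timeline finishes.
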(event `self.ReceiveTick`
  (params (DeltaSeconds :type "Float (single-precision)"))
  (`self.RotateWidgetToPlayer`))

(event `RotateWidgetToPlayer`
  (bind (_returnvalue_roll _returnvalue_pitch _returnvalue_yaw) (`KismetMathLibrary.BreakRotator` (`KismetMathLibrary.FindLookAtRotation` (`SceneComponent.K2_GetComponentLocation` (`self.ParentScene`)) (`self.K2_GetActorLocation` (`self.PlayerRef`)))))
  (bind (_returnvalue_roll_2 _returnvalue_pitch_2 _returnvalue_yaw_2) (`KismetMathLibrary.BreakRotator` (`KismetMathLibrary.FindLookAtRotation` (`SceneComponent.K2_GetComponentLocation` (`self.WidgetHolder`)) (`self.K2_GetActorLocation` (`self.PlayerRef`)))))
  ; Comment
  (`/Engine/EditorBlueprintResources/StandardMacros.IsValid` (`self.ParentScene`)
    (:`Is Valid`
      (`SceneComponent.K2_SetWorldRotation` (`self.ParentScene`) (`KismetMathLibrary.MakeRotator` _returnvalue_roll _returnvalue_pitch _returnvalue_yaw) false false))
    (:`Is Not Valid`
      (`|ExecutionSequence`
        (:`then_0`
          (`SceneComponent.K2_SetWorldRotation` (`self.WidgetHolder`) (`KismetMathLibrary.MakeRotator` _returnvalue_roll_2 0.0 _returnvalue_yaw_2) false false))
        (:`then_1`
          (`/Engine/EditorBlueprintResources/StandardMacros.DoOnce` false
            (:`Completed`
              (`|ExecutionSequence`
                (:`then_0`
                  (bind (_direction _newtrack_0) (`Timeline|Timeline` :!via `Reverse`)
                    (:`Update`
                      (`SceneComponent.SetRelativeScale3D` (`self.DmgWidget`) (`KismetMathLibrary.MakeVector` _newtrack_0 _newtrack_0 _newtrack_0)))))
                (:`then_1`
                  (bind (_direction_2 _newtrack_0_2) (`Timeline|Timeline_0` :!via `PlayFromStart`)
                    (:`Update`
                      (`Widget.SetRenderOpacity` (`WidgetComponent.GetWidget` (`self.DmgWidget`)) _newtrack_0_2))
                    (:`Finished`
                      (`self.K2_DestroyActor`))))))))))))

(fn `UserConstructionScript`)