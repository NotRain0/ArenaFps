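; BP_LaserActor is a visual laser with beam and impact effect components, driven by the sight data of its parent reference.
; ActivateLaser and DeactivateLaser toggle both effects and the IsOn flag.
; While on, the custom FalseTick event, used in place of Event Tick, moves the beam end and impact to the parent's sight hit location.
; The impact shows only while the parent has a valid actor in sight.
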(event `DeactivateLaser`
  (`ActorComponent.Deactivate` (`self.N_Laser`))
  (`ActorComponent.Deactivate` (`self.N_LaserImpact`))
  (`SceneComponent.SetVisibility` (`self.N_LaserImpact`) false false)
  (`SceneComponent.SetVisibility` (`self.N_Laser`) false false)
  (set `self.IsOn` false))

(event `ActivateLaser`
  (`ActorComponent.Activate` (`self.N_Laser`) false)
  (`ActorComponent.Activate` (`self.N_LaserImpact`) false)
  (`SceneComponent.SetVisibility` (`self.N_Laser`) true false)
  (set `self.IsOn` true))

(event `FalseTick`
  (bind _n_laserimpact (`self.N_LaserImpact`))
  (bind _actorsighthitlocation (`/Game/Blueprint/A_Rework/BP_PlayerCharNew.ActorSightHitLocation` (`self.ParentRef`)))
  (if (`self.IsOn`)
    (`FXSystemComponent.SetVectorParameter` (`self.N_Laser`) "BeamEnd" _actorsighthitlocation)
    (`SceneComponent.SetVisibility` _n_laserimpact (`KismetSystemLibrary.IsValid` (`/Game/Blueprint/A_Rework/BP_PlayerCharNew.ActorInSight` (`self.ParentRef`))) false)
    (`SceneComponent.K2_SetWorldLocation` _n_laserimpact _actorsighthitlocation false false)))

(fn `UserConstructionScript`)