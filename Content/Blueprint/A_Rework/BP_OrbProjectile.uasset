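; Orb projectile that scales up on spawn, flies forward by moving on Tick after StartMoving, and self-destroys 10 seconds after the scale-up.
; Overlapping an untagged actor triggers Explode, which stops it, enlarges it fifteenfold and restyles its Niagara effect.
; After that timeline it damages overlapping BP_BaseEnemyNew actors, with burning ones taking a bonus scaled by the total enemy count, then fades out and destroys itself.
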(event `self.ReceiveBeginPlay`
  ; Comment
  (bind (_direction _newtrack_0) (`Timeline|Timeline`)
    (:`Update`
      (`SceneComponent.SetRelativeScale3D` (`self.Scene`) (`KismetMathLibrary.MakeVector` _newtrack_0 _newtrack_0 _newtrack_0)))
    (:`Finished`
      (`KismetSystemLibrary.Delay` 10.0)
      (`self.K2_DestroyActor`))))

(event `self.Sphere.OnComponentBeginOverlap`
  (params (OverlappedComponent :type "PrimitiveComponent Object Reference") (OtherActor :type "Actor Object Reference") (OtherComp :type "PrimitiveComponent Object Reference") (OtherBodyIndex :type Integer) (bFromSweep :type Boolean) (SweepResult :type "HitResult Structure (by ref)"))
  (if (and (`self.canMove`) (== (`KismetArrayLibrary.Array_Length` (`Actor.Tags` OtherActor)) 0))
    (`KismetSystemLibrary.PrintString` (`KismetStringLibrary.Concat_StrStr` "ball hit : " (`KismetSystemLibrary.GetDisplayName` OtherActor)))
    (`self.Explode`)))

(event `StartMoving`
  (params (Forward :type "Rotator Structure"))
  ; Comment
  (`self.K2_SetActorRotation` Forward)
  (set `self.canMove` true))

(event `self.ReceiveTick`
  (params (DeltaSeconds :type "Float (single-precision)"))
  ; Comment
  (if (`self.canMove`)
    (`self.K2_SetActorLocation` (+ (`self.K2_GetActorLocation`) (* DeltaSeconds (`self.Speed`) (`self.GetActorForwardVector`))))))

(event `Explode`
  (bind _niagara (`self.Niagara`))
  (bind _overlappingactors (`PrimitiveComponent.GetOverlappingActors` (`self.Sphere`) "/Game/Blueprint/A_Rework/BP_BaseEnemyNew.BP_BaseEnemyNew_C"))
  (bind _returnvalue (* 15 (`self.BaseScale`)))
  ; Comment
  (`|ExecutionSequence`
    (:`then_0`
      (set `self.BaseScale` (`SceneComponent.RelativeScale3D` (`self.Scene`)))
      (set `self.canMove` false)
      (`NiagaraComponent.SetVariableVec2` (`self.Niagara`) "SizeMin" (125.0 125.0))
      (`NiagaraComponent.SetVariableVec2` _niagara "SizeMax" (125.0 125.0))
      (`NiagaraComponent.SetVariableLinearColor` _niagara "Color" (make `LinearColor` 0.0 0.0 5.0 1.0)))
    (:`then_1`
      (bind (_direction _newtrack_0) (`Timeline|Timeline_0` :!via `PlayFromStart`)
        (:`Update`
          (`SceneComponent.SetRelativeScale3D` (`self.Scene`) (`KismetMathLibrary.VLerp` _returnvalue _returnvalue _newtrack_0)))
        (:`Finished`
          (for _array_element _overlappingactors
            (bind _asbp_base_enemy_new (cast `/Game/Blueprint/A_Rework/BP_BaseEnemyNew` _array_element))
            (`/Game/Blueprint/A_Rework/BP_BaseEnemyNew.ChangeHealth` _asbp_base_enemy_new (`KismetMathLibrary.SelectFloat` (+ (* (`KismetArrayLibrary.Array_Length` _overlappingactors) (`self.DamageByBurningEnemiesInAot`)) (`self.DamageBase`)) (`self.DamageBase`) (`/Game/Blueprint/A_Rework/BP_BaseEnemyNew.IsBurning` _asbp_base_enemy_new)) false false))
          (bind (_direction_2 _newtrack_0_2) (`Timeline|Timeline_1` :!via `PlayFromStart`)
            (:`Update`
              (`FXSystemComponent.SetFloatParameter` (`self.Niagara`) "Alpha" (`KismetMathLibrary.Lerp` 1.0 0.0 _newtrack_0_2)))
            (:`Finished`
              (`self.K2_DestroyActor`))))))))

(fn `UserConstructionScript`)