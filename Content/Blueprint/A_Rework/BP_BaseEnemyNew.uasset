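; Base enemy Blueprint that handles health, floating damage numbers, laser-triggered burning and death.
; ChangeHealth clamps health and feeds a damage widget whose scale and fade timelines use a retriggerable delay, shorter for laser hits, to hide it.
; Enough accumulated laser damage activates a fire effect until a retriggerable delay expires.
; The text lives on a separate spawned actor, reattached on death to a player-facing BP_Cross before the enemy is destroyed.
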(event `DisplayHitDamage`
  ; Display Damage
  (set `self.DamagedRecently` true)
  (`|ExecutionSequence`
    (:`then_0`
      (bind (_direction _newtrack_0) (`Timeline|FadeText` :!via `Stop` :!label _label)
        (:`Update`
          (`Widget.SetRenderOpacity` (`self.TextWidgetRef`) _newtrack_0))
        (:`Finished`
          (set `self.DmgFromLaser` 0.0)
          (set `/Game/Blueprint/A_Rework/WBP_DmgTextNew.DmgCumulated` 0.0 (`self.TextWidgetRef`)))))
    (:`then_1`
      (`Widget.SetRenderOpacity` (`self.TextWidgetRef`) 1.0)
      (bind (_direction_2 _newtrack_0_2) (`Timeline|HandleDamageAmountSize` :!label _label_2)
        (:`Update`
          (`SceneComponent.SetRelativeScale3D` (`self.DmgWidget`) (`KismetMathLibrary.MakeVector` _newtrack_0_2 _newtrack_0_2 _newtrack_0_2)))))))

(event `StartBurning`
  ; Comment
  (`|ExecutionSequence`
    (:`then_0`
      (`KismetSystemLibrary.RetriggerableDelay` (`self.TimeBeforeResetBurn`))
      (`ActorComponent.Deactivate` (`self.NS_Fire`))
      (set `self.IsBurning` false))
    (:`then_1`
      (if (not (`self.IsBurning`))
        (set `self.IsBurning` true)
        (`ActorComponent.Activate` (`self.NS_Fire`) true)))))

(event `HideHitDamage`
  ; Display Damage
  (set `self.DamagedRecently` false)
  (`|ExecutionSequence`
    (:`then_0`
      (goto _label_2 :!via `Reverse`))
    (:`then_1`
      (goto _label))))

(event `self.ReceiveBeginPlay`
  ; Comment
  (set `self.currentHealth` (`self.maxHealth`))
  (`self.SetDamageWidget`))

(event `ChangeHealth`
  (params (Amount :type "Float (double-precision)") (FromLaser :type Boolean) (HitInHead :type Boolean))
  (bind _returnvalue (* Amount -1.0))
  ;[1 0 0 0.5] Comment
  (`|ExecutionSequence`
    (:`then_0`
      (if (not (`self.DamagedRecently`))
        (`self.DisplayHitDamage`))
      (bind _output_get (set `self.currentHealth` (`KismetMathLibrary.FClamp` (+ Amount (`self.currentHealth`)) 0.0 (`self.maxHealth`))))
      (if (<= _output_get 0.0)
        (`self.CustomDeath`)
        (else
          (if FromLaser
            (bind _output_get_2 (set `self.DmgFromLaser` (+ _returnvalue (`self.DmgFromLaser`)))))
          (`/Game/Blueprint/A_Rework/WBP_DmgTextNew.ChangeAmountWidg` (`self.TextWidgetRef`) HitInHead _returnvalue (`/Game/Blueprint/A_Rework/BP_PlayerCharNew.DeltaTimeSave` (`self.PlayerRef`)))
          (if (>= _output_get_2 (`self.DmgFromLaserBeforeBurning`))
            (`self.StartBurning`)))))
    (:`then_1`
      (`KismetSystemLibrary.RetriggerableDelay` (`KismetMathLibrary.SelectFloat` 0.1 1.0 FromLaser))
      (`self.HideHitDamage`))))

(event `CustomDeath`
  (bind _returnvalue (`self.GetTransform`))
  (bind (_returnvalue_roll _returnvalue_pitch _returnvalue_yaw) (`KismetMathLibrary.BreakRotator` (`KismetMathLibrary.FindLookAtRotation` (`self.K2_GetActorLocation`) (`self.K2_GetActorLocation` (`self.PlayerRef`)))))
  ; Comment
  (bind _returnvalue_2 (`|SpawnActorFromClass` "/Game/Blueprint/A_Rework/BP_Cross.BP_Cross_C" (`KismetMathLibrary.MakeTransform` (`KismetMathLibrary.MakeVector` (.x (.location _returnvalue)) (.y (.location _returnvalue)) (- (.z (.location _returnvalue)) (`CapsuleComponent.CapsuleHalfHeight` (`self.CapsuleComponent`)))) (`KismetMathLibrary.MakeRotator` _returnvalue_roll 0.0 _returnvalue_yaw)) "AlwaysSpawn" "MultiplyWithRoot" null null))
  (`self.K2_AttachToComponent` (`self.TextActor`) (`/Game/Blueprint/A_Rework/BP_Cross.Center` _returnvalue_2) "None" "KeepWorld" "KeepWorld" "KeepWorld" true)
  (`self.K2_DestroyActor`))

(fn `SetDamageWidget`
  (bind _textactor (`self.TextActor`))
  (bind _returnvalue (`GameplayStatics.GetActorOfClass` "/Game/Blueprint/A_Rework/BP_PlayerCharNew.BP_PlayerCharNew_C"))
  (set `self.PlayerRef` _returnvalue)
  (bind _returnvalue_2 (`|SpawnActorFromClass` "/Game/Blueprint/A_Rework/TextHolderActor.TextHolderActor_C" (`SceneComponent.K2_GetComponentToWorld` (`self.TextSceneHolder`)) "Undefined" "MultiplyWithRoot" null null))
  (bind _output_get (set `self.TextActor` _returnvalue_2))
  (`self.K2_AttachToComponent` _output_get (`self.TextAnchor`) "None" "KeepWorld" "KeepWorld" "KeepWorld" true)
  (bind _output_get_2 (set `self.DmgWidget` (`/Game/Blueprint/A_Rework/TextHolderActor.DmgWidget` (`self.TextActor`))))
  (bind _aswbp_dmg_text_new (cast `/Game/Blueprint/A_Rework/WBP_DmgTextNew` (`WidgetComponent.GetWidget` _output_get_2)))
  (bind _output_get_3 (set `self.TextWidgetRef` _aswbp_dmg_text_new))
  (`Widget.SetRenderOpacity` _output_get_3 1.0)
  (set `/Game/Blueprint/A_Rework/TextHolderActor.PlayerRef` (`self.PlayerRef`) _textactor)
  (set `/Game/Blueprint/A_Rework/TextHolderActor.ParentScene` (`self.TextSceneHolder`) _textactor)
  (`self.SetActorTickEnabled` (`self.TextActor`) true))

(fn `UserConstructionScript`)