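; Brazier actor with a world-space health bar and a visual effect for killing enemies in range.
; BeginPlay caches the player and the health widget, then refreshes the bar from CurrentHealth over MaxHealth in a looping short Delay.
; Tick rotates the widget to face the player.
; KillEnemyinRangeBlueprintVisual shows a sphere scaled by a timeline, then hides and resets it; the event handles only visuals.
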(event `self.ReceiveBeginPlay`
  (`|ExecutionSequence`
    (:`then_0`
      (bind _returnvalue (`GameplayStatics.GetActorOfClass` "/Game/Blueprint/A_Rework/BP_PlayerCharNew.BP_PlayerCharNew_C"))
      (set `self.PlayerRef` _returnvalue))
    (:`then_1`
      (bind _asbp_brasier_health_v0 (cast `/Game/Blueprint/Brasier/BP_BrasierHealthV0` (`WidgetComponent.GetWidget` (`self.Widget`))))
      (bind _output_get (set `self.refWidgetV0` _asbp_brasier_health_v0))
      (`/Engine/EditorBlueprintResources/StandardMacros.IsValid` _output_get
        (:`Is Valid`
          (`KismetSystemLibrary.Delay` 0.2 :!label _label)
          (`ProgressBar.SetPercent` (`/Game/Blueprint/Brasier/BP_BrasierHealthV0.ProgressBar_47` (`self.refWidgetV0`)) (/ (`self.currentHealth`) (`self.maxHealth`)))
          (goto _label))))))

(event `self.ReceiveTick`
  (params (DeltaSeconds :type "Float (single-precision)"))
  (bind _widget (`self.Widget`))
  (`SceneComponent.K2_SetWorldRotation` _widget (`KismetMathLibrary.FindLookAtRotation` (`SceneComponent.K2_GetComponentLocation` _widget) (`self.K2_GetActorLocation` (`self.PlayerRef`))) false false))

(event `self.KillEnemyInRangeBlueprintVisual`
  (bind _explosionsphere (`self.ExplosionSphere`))
  (`SceneComponent.SetHiddenInGame` (`self.ExplosionSphere`) false false)
  (bind (_direction _newtrack_0) (`Timeline|Timeline` :!via `PlayFromStart`)
    (:`Update`
      (`SceneComponent.SetRelativeScale3D` (`self.ExplosionSphere`) (`KismetMathLibrary.MakeVector` _newtrack_0 _newtrack_0 _newtrack_0)))
    (:`Finished`
      (`SceneComponent.SetHiddenInGame` _explosionsphere true false)
      (`SceneComponent.SetRelativeScale3D` _explosionsphere (1.0 1.0 1.0)))))

(fn `UserConstructionScript`)